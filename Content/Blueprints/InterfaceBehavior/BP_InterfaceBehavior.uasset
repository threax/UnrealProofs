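; BP_InterfaceBehavior is a test Blueprint that exercises interface message behavior on two object types, BP_Thing and BP_NotThing.
; On BeginPlay it constructs one of each and passes them repeatedly, in mixed order, to ThingEvent.
; ThingEvent validates the object, sends it the ThingTesterIsThingMessage call and prints whether it is a thing based on the returned boolean.
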(event Custom|ThingEvent
  (params (Test :type Object%20Object%20Reference))
  (Utilities|IsValid Test
    (:Is%20Valid
      (bind _itisthething (Class|BPIThingTester|ThingTesterIsThing(Message) Test))
      (if _itisthething
        (Development|PrintString "It is a thing!")
        (else
          (Development|PrintString "It is not a thing!"))))))

(event EventBeginPlay
  (bind _returnvalue (Game|ConstructObjectfromClass "/Game/Blueprints/InterfaceBehavior/BP_Thing.BP_Thing_C"))
  (CallFunction|ThingEvent _returnvalue)
  (bind _returnvalue_2 (Game|ConstructObjectfromClass "/Game/Blueprints/InterfaceBehavior/BP_NotThing.BP_NotThing_C"))
  (CallFunction|ThingEvent _returnvalue_2)
  (CallFunction|ThingEvent _returnvalue)
  (CallFunction|ThingEvent _returnvalue_2)
  (CallFunction|ThingEvent _returnvalue_2))

(fn ConstructionScript)