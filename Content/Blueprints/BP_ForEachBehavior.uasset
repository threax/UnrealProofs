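; BP_ForEachBehavior is a test Blueprint that demonstrates how ForEach loops evaluate a pure function supplying their array.
; On BeginPlay it loops over PureArrayAccessor twice: first as a pure node re-evaluated during iteration, then with exec pins so it runs only once.
; The accessor increments a counter and prints it before returning ArrayOfThings, so the printed output exposes the repeated calls alongside each element.
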(event EventBeginPlay
  (Utilities|FlowControl|Sequence
    (:then_0
      ;[0.15 0.15 0.15 0.5] Pure function called each iteration
      (for _array_element (CallFunction|PureArrayAccessor)
        (Development|PrintText (Utilities|Text|FormatText "Array element {element}" _array_element))))
    (:then_1
      ;[0.15 0.15 0.15 0.5] Pure function called with exec pins. Will only be called once.
      (Development|PrintText "Starting exec loop")
      (bind _arrayofthings (CallFunction|PureArrayAccessor))
      (for _array_element_2 _arrayofthings
        (Development|PrintText (Utilities|Text|FormatText "Exec Pure Array element {element}" _array_element_2))))))

(fn ConstructionScript)

(fn PureArrayAccessor
  (Math|Integer|IncrementInt (Variables|Default|GetPureAccessorCount)
    (:%20%20
      (Development|PrintText (Utilities|Text|FormatText "Accessed Array through Pure Function {count} times." (Variables|Default|GetPureAccessorCount)))
      (return (Variables|Default|GetArrayOfThings)))))