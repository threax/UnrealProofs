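; BP_PureFunctionBehavior is a test Blueprint that demonstrates how often a pure function is evaluated.
; PureThing increments and returns PureCounter, so each evaluation is visible in its result.
; On BeginPlay, a sequence first prints three separate calls expecting an increasing count.
; It then prints one call's result three times, expecting the same next value, with expected and actual values in each message.
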(event EventBeginPlay
  (Utilities|FlowControl|Sequence
    (:then_0
      (Development|PrintText (Utilities|Text|FormatText "Pure call 1 expect 1 {result}" (CallFunction|PureThing)))
      (Development|PrintText (Utilities|Text|FormatText "Pure call 2 expect 2 {result}" (CallFunction|PureThing)))
      (Development|PrintText (Utilities|Text|FormatText "Pure call 3 expect 3 {result}" (CallFunction|PureThing))))
    (:then_1
      (bind _count (CallFunction|PureThing))
      (Development|PrintText (Utilities|Text|FormatText "Exec Pure call 1 expect 4 got {result}" _count))
      (Development|PrintText (Utilities|Text|FormatText "Exec Pure call 2 expect 4 got {result}" _count))
      (Development|PrintText (Utilities|Text|FormatText "Exec Pure call 3 expect 4 got {result}" _count)))))

(fn ConstructionScript)

(fn PureThing
  (Math|Integer|IncrementInt (Variables|Default|GetPureCounter)
    (:%20%20
      (return (Variables|Default|GetPureCounter)))))